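; MP5 automatic weapon for the first-person pawn, with aim-down-sights, montage-driven reload and ammo state saved on unequip.
; Fire loops through a Gate and retriggerable delay, spending ammo and spawning decals, tracers, sound and muzzle flash.
; LineTrace shoots from the camera with random spread set by aim state and movement speed.
; Hits push Movable physics props and launch zombie pawns; no damage is applied here.
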(event EventUnequip
  (Variables|/Game/Blueprints/Player/FPSPawn_BP.FPSPawn_BP_C|SetPrimaryWeapon (.AsFPSPawn%20BP (Utilities|Casting|CastToFPSPawn_BP (Game|GetPlayerCharacter 0))) (Utilities|Struct|MakeGunData "NewEnumerator2" "Weapon_MP5_C" (Variables|Default|GetAmmoCount) (Variables|Default|GetMaxAmmo) (Variables|Default|GetReloadTime) (Variables|Default|GetBulletSpread))))

(event EventStopFiring
  (bind _returnvalue (Game|GetPlayerCharacter 0))
  (bind _returnvalue_2 (Game|GetPlayerCharacter 0))
  (bind _asfpspawn_bp (Utilities|Casting|CastToFPSPawn_BP _returnvalue_2))
  (bind _asfpspawn_bp_2 (Utilities|Casting|CastToFPSPawn_BP _returnvalue))
  (bind _mesh1p (Variables|/Game/Blueprints/Player/FPSPawn_BP.FPSPawn_BP_C|GetMesh1P _asfpspawn_bp_2))
  ;[1 1 1] For Automatic Weapon
  (Utilities|FlowControl|Gate true) ; enters at Close
)

(event EventFire
  (bind _returnvalue (Game|GetPlayerCharacter 0))
  (bind _returnvalue_2 (Game|GetPlayerCharacter 0))
  (bind _asfpspawn_bp (Utilities|Casting|CastToFPSPawn_BP _returnvalue_2))
  (bind _asfpspawn_bp_2 (Utilities|Casting|CastToFPSPawn_BP _returnvalue))
  (bind _mesh1p (Variables|/Game/Blueprints/Player/FPSPawn_BP.FPSPawn_BP_C|GetMesh1P _asfpspawn_bp_2))
  ;[1 1 1] For Automatic Weapon
  (Utilities|FlowControl|Sequence
    (:then_0
      (goto _label Open))
    (:then_1
      (Utilities|FlowControl|Gate true :!label _label
        (:Exit
          (Utilities|FlowControl|Sequence
            (:then_0
              (if (not (Variables|/Game/Blueprints/Player/FPSPawn_BP.FPSPawn_BP_C|GetIsReloading _asfpspawn_bp))
                (if (> (Variables|Default|GetAmmoCount) 0)
                  (CallFunction|AmmoCheck)
                  (bind (_muzzleloc _impactpoint) (CallFunction|LineTrace))
                  (CallFunction|SpawnDecalTracer _muzzleloc _impactpoint _impactpoint)
                  (if (Variables|/Game/Blueprints/Player/FPSPawn_BP.FPSPawn_BP_C|GetAimDownSight _asfpspawn_bp_2)
                    (Animation|Montage|PlayMontage _mesh1p "/Game/FPSPawn/Animations/Arms_MP5_ADS_Fire_anim_Montage.Arms_MP5_ADS_Fire_anim_Montage"
                      (:then
                        _))
                    (else
                      (Animation|Montage|PlayMontage _mesh1p "/Game/FPSPawn/Animations/Arms_MP5_Fire_anim_Montage.Arms_MP5_Fire_anim_Montage"
                        (:then
                          _))))
                  (Utilities|MuzzleFlash)
                  (else
                    (Audio|PlaySoundatLocation "/Game/FPSPawn/SoundFX/DryFire.DryFire" (Transformation|GetWorldLocation (Variables|/Game/Blueprints/Player/FPSPawn_BP.FPSPawn_BP_C|GetFirstPersonCamera _asfpspawn_bp)) "0, 0, 0" 1.0 1.0 0.0 "/Game/FPSPawn/SoundFX/AK_Attenuation.AK_Attenuation" "/Game/FPSPawn/SoundFX/AK_Concurrency.AK_Concurrency" 0)))))
            (:then_1
              (Utilities|FlowControl|RetriggerableDelay 0.12)
              (goto _label))))))))

(event EventReload
  (bind _returnvalue (Game|GetPlayerCharacter 0))
  (bind _asfpspawn_bp (Utilities|Casting|CastToFPSPawn_BP _returnvalue))
  (if (< (Variables|Default|GetAmmoCount) (Variables|Default|GetMaxAmmo))
    (Utilities|FlowControl|DoOnce false :!label _label
      (:Completed
        (Variables|/Game/Blueprints/Player/FPSPawn_BP.FPSPawn_BP_C|SetIsReloading _asfpspawn_bp true)
        (Animation|Montage|MontagePlay (Components|SkeletalMesh|GetAnimInstance (Variables|/Game/Blueprints/Player/FPSPawn_BP.FPSPawn_BP_C|GetMesh1P _asfpspawn_bp)) "/Game/FPSPawn/Animations/Arms_MP5_Reload_anim_Montage.Arms_MP5_Reload_anim_Montage" 1.0 "MontageLength" 0.0 true)
        (Components|Animation|PlayAnimation (Variables|Default|GetPrimaryWeapon) "/Game/FPSPawn/Animations/MP5_Reload_anim.MP5_Reload_anim" false)
        (Utilities|FlowControl|Delay (Variables|Default|GetReloadTime))
        (Variables|Default|SetAmmoCount (Variables|Default|GetMaxAmmo))
        (Variables|/Game/Blueprints/Player/FPSPawn_BP.FPSPawn_BP_C|SetIsReloading _asfpspawn_bp false)
        (goto _label Reset)))))

(event EventADS
  (params (Toggle :type Boolean))
  (bind _returnvalue (Game|GetPlayerCharacter 0))
  (bind _asfpspawn_bp (Utilities|Casting|CastToFPSPawn_BP _returnvalue))
  (bind _firstpersoncamera (Variables|/Game/Blueprints/Player/FPSPawn_BP.FPSPawn_BP_C|GetFirstPersonCamera _asfpspawn_bp))
  (bind _mesh1p (Variables|/Game/Blueprints/Player/FPSPawn_BP.FPSPawn_BP_C|GetMesh1P _asfpspawn_bp))
  (if Toggle
    (bind _float (Timeline|Timeline_0 PlayFromStart)
      (:Update
        (Camera|SetFieldOfView _firstpersoncamera (Math|Float|Lerp 9e+01 45.0 _float))
        (Transformation|SetRelativeTransform _mesh1p (Math|Transform|MakeTransform (Math|Vector|Lerp(Vector) "1.600000,7.800000,-24.000000" "1.600000,0.000000,-16.500000" _float) "0,-1.050000, 0" "1,1,1") false false)))
    (else
      (bind _float_2 (Timeline|Timeline_1 PlayFromStart)
        (:Update
          (Camera|SetFieldOfView _firstpersoncamera (Math|Float|Lerp 45.0 9e+01 _float_2))
          (Transformation|SetRelativeTransform _mesh1p (Math|Transform|MakeTransform (Math|Vector|Lerp(Vector) "1.600000,0.000000,-16.500000" "1.600000,7.800000,-24.000000" _float_2) "0.000000,6.400000, 0" "1,1,1") false false))))))

(fn ConstructionScript
  (|CallParentFunction)
  (Variables|Default|SetMaxAmmo 30)
  (Variables|Default|SetAmmoCount 30)
  (Variables|Default|SetReloadTime 2.0)
  (Variables|Default|SetBulletSpread 5e+02)
  (Variables|Default|SetName "NewEnumerator2")
  (Variables|Default|SetVariableMode false)
  (Variables|Default|SetStrenght 2e+02)
  (Variables|Default|SetStrenghtKnockback 7.0))

(fn AmmoCheck
  (bind _returnvalue (Math|Random|RandomFloatinRange 0.7 1.2))
  (Math|Integer|DecrementInt (Variables|Default|GetAmmoCount)
    (:%20%20
      (Audio|PlaySoundatLocation "/Game/FPSPawn/SoundFX/Gunshot.Gunshot" (Transformation|GetWorldLocation (Variables|/Game/Blueprints/Player/FPSPawn_BP.FPSPawn_BP_C|GetFirstPersonCamera (.AsFPSPawn%20BP (Utilities|Casting|CastToFPSPawn_BP (Game|GetPlayerCharacter 0))))) "0, 0, 0" (+ _returnvalue 2.5) _returnvalue 0.0 "/Game/FPSPawn/SoundFX/AK_Attenuation.AK_Attenuation" "/Game/FPSPawn/SoundFX/AK_Concurrency.AK_Concurrency" 0)
      (Components|Animation|PlayAnimation (Variables|Default|GetPrimaryWeapon) "/Game/FPSPawn/Animations/AK_Fire_anim.AK_Fire_anim" false))))

(fn LineTrace
  (bind _returnvalue (Game|GetPlayerCharacter 0))
  (bind _muzzle (Variables|Default|GetMuzzle))
  (bind _returnvalue_2 (Transformation|GetWorldLocation _muzzle))
  (bind _asfpspawn_bp (Utilities|Casting|CastToFPSPawn_BP _returnvalue))
  (bind _firstpersoncamera (Variables|/Game/Blueprints/Player/FPSPawn_BP.FPSPawn_BP_C|GetFirstPersonCamera _asfpspawn_bp))
  (bind _charactermovement (Variables|/Script/Engine.Character|GetCharacterMovement _asfpspawn_bp))
  (bind _returnvalue_3 (Pawn|Components|CharacterMovement|GetLastUpdateVelocity _charactermovement))
  (bind _returnvalue_4 (Transformation|GetWorldLocation _firstpersoncamera))
  (bind _returnvalue_5 (Math|Vector|VectorLength _returnvalue_3))
  (bind _returnvalue_6 (<= _returnvalue_5 1e+02))
  (if (Variables|/Game/Blueprints/Player/FPSPawn_BP.FPSPawn_BP_C|GetAimDownSight _asfpspawn_bp)
    (if _returnvalue_6
      (Variables|Default|SetBulletSpread 0.0)
      (else
        (Variables|Default|SetBulletSpread 2.5e+02 :!label _label)))
    (elif _returnvalue_6
      (goto _label)
      (else
        (Variables|Default|SetBulletSpread 5e+02))))
  (bind _outhit (Collision|LineTraceByChannel (+ _returnvalue_4 (Variables|Default|GetAimOffset)) (+ (+ _returnvalue_4 (* (Math|Vector|GetForwardVector _firstpersoncamera) 2e+04)) (Math|Vector|MakeVector (Math|Random|RandomFloatinRange (* (Variables|Default|GetBulletSpread) -1.0) (Variables|Default|GetBulletSpread)) (Math|Random|RandomFloatinRange (* (Variables|Default|GetBulletSpread) -1.0) (Variables|Default|GetBulletSpread)) (Math|Random|RandomFloatinRange (* (Variables|Default|GetBulletSpread) -1.0) (Variables|Default|GetBulletSpread)))) "TraceTypeQuery1" false 0 "None")) ; Camera Shot
  (if (.bBlockingHit (Collision|BreakHitResult _outhit))
    ;[1 1 1] Impulse to props
    (Utilities|PropsKnockback (.ImpactPoint (Collision|BreakHitResult _outhit)) (.ImpactNormal (Collision|BreakHitResult _outhit)) (.HitActor (Collision|BreakHitResult _outhit)) (.HitComponent (Collision|BreakHitResult _outhit))
      (:True
        (Collision|LineTraceByChannel _returnvalue_2 (.ImpactPoint (Collision|BreakHitResult _outhit)) "TraceTypeQuery1" false 0 "None" true "(R=0.000000,G=1.000000,B=0.000000,A=1.000000)") ; Gun Shot
      )
      (:false
        _)))
  (return _returnvalue_2 (.ImpactPoint (Collision|BreakHitResult _outhit))))

(fn SpawnDecalTracer
  (params (Location :type Vector) (SpawnTransformLoc :type Vector) (Impact%20Point :type Vector))
  (Game|SpawnActorfromClass "/Game/Blueprints/Weapons/BulletDecal_BP.BulletDecal_BP_C" (Math|Transform|MakeTransform SpawnTransformLoc (Math|Conversions|RotationFromXVector Impact%20Point) "0.025000,0.025000,0.025000") "Undefined" 0 0)
  (if true
    (Game|SpawnActorfromClass "/Game/Blueprints/Weapons/TracerRound_BP.TracerRound_BP_C" (Math|Transform|MakeTransform Location (Transformation|GetWorldRotation (Variables|/Game/Blueprints/Player/FPSPawn_BP.FPSPawn_BP_C|GetFirstPersonCamera (.AsFPSPawn%20BP (Utilities|Casting|CastToFPSPawn_BP (Game|GetPlayerCharacter 0))))) "0.050000,0.050000,0.050000") "Undefined" 0 0))
  (return))