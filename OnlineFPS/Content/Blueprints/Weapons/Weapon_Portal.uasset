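; Portal gun weapon for the FPS pawn: Fire places Portal A and ADS places Portal B where a camera line trace hits.
; Each shot replaces that portal on the pawn, orients it to the surface normal and sets both portals' render materials once the pair exists.
; Shots play AK arm montages and a muzzle flash.
; Ammo is zeroed; the ammo-decrement and knockback/damage paths are left unconnected.
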(event Custom|Line%20Trace
  (bind _returnvalue (Game|GetPlayerCharacter 0))
  (bind _asfpspawn_bp (Utilities|Casting|CastToFPSPawn_BP _returnvalue))
  (bind _mesh1p (Variables|/Game/Blueprints/Player/FPSPawn_BP.FPSPawn_BP_C|GetMesh1P _asfpspawn_bp))
  (bind (_muzzleloc _impactpoint _impactnormal) (CallFunction|LineTrace))
  (CallFunction|SpawnPortalA _muzzleloc _impactpoint _impactpoint _impactnormal)
  (if (Variables|/Game/Blueprints/Player/FPSPawn_BP.FPSPawn_BP_C|GetAimDownSight _asfpspawn_bp)
    (Animation|Montage|PlayMontage _mesh1p "/Game/FPSPawn/Animations/Arms_AK_ADS_Fire_anim_Montage.Arms_AK_ADS_Fire_anim_Montage"
      (:then
        _))
    (else
      (Animation|Montage|PlayMontage _mesh1p "/Game/FPSPawn/Animations/Arms_AK_Fire_Montage.Arms_AK_Fire_Montage"
        (:then
          _))))
  (Utilities|MuzzleFlash))

(event EventUnequip
  (Variables|/Game/Blueprints/Player/FPSPawn_BP.FPSPawn_BP_C|SetPrimaryWeapon (.AsFPSPawn%20BP (Utilities|Casting|CastToFPSPawn_BP (Game|GetPlayerCharacter 0))) (Utilities|Struct|MakeGunData "NewEnumerator5" "Weapon_Portal_C" (Variables|Default|GetAmmoCount) (Variables|Default|GetMaxAmmo) (Variables|Default|GetReloadTime) (Variables|Default|GetBulletSpread))))

(event EventStopFiring
  (bind _returnvalue (Game|GetPlayerCharacter 0))
  (bind _asfpspawn_bp (Utilities|Casting|CastToFPSPawn_BP _returnvalue))
  ;[0.125 0 1] For Automatic Weapon
  (Utilities|FlowControl|Gate true) ; enters at Close
)

(event EventFire
  ;[0.125 0 1] For Automatic Weapon
  (CallFunction|LineTrace))

(event EventReload
  (bind _returnvalue (Game|GetPlayerCharacter 0))
  (bind _asfpspawn_bp (Utilities|Casting|CastToFPSPawn_BP _returnvalue))
  (if (< (Variables|Default|GetAmmoCount) (Variables|Default|GetMaxAmmo))
    (Utilities|FlowControl|DoOnce false :!label _label
      (:Completed
        (Variables|/Game/Blueprints/Player/FPSPawn_BP.FPSPawn_BP_C|SetIsReloading _asfpspawn_bp true)
        (Animation|Montage|MontagePlay (Components|SkeletalMesh|GetAnimInstance (Variables|/Game/Blueprints/Player/FPSPawn_BP.FPSPawn_BP_C|GetMesh1P _asfpspawn_bp)) "/Game/FPSPawn/Animations/Arms_AK_Reload_Montage.Arms_AK_Reload_Montage" 1.0 "MontageLength" 0.0 true)
        (Components|Animation|PlayAnimation (Variables|Default|GetPrimaryWeapon) "/Game/FPSPawn/Animations/AK_Reload_anim_Montage.AK_Reload_anim_Montage" false)
        (Utilities|FlowControl|Delay (Variables|Default|GetReloadTime))
        (Variables|Default|SetAmmoCount (Variables|Default|GetMaxAmmo))
        (Variables|/Game/Blueprints/Player/FPSPawn_BP.FPSPawn_BP_C|SetIsReloading _asfpspawn_bp false)
        (goto _label Reset)))))

(event EventADS
  (params (Toggle :type Boolean))
  (bind _returnvalue (Game|GetPlayerCharacter 0))
  (bind _asfpspawn_bp (Utilities|Casting|CastToFPSPawn_BP _returnvalue))
  (bind _mesh1p (Variables|/Game/Blueprints/Player/FPSPawn_BP.FPSPawn_BP_C|GetMesh1P _asfpspawn_bp))
  (bind (_muzzleloc _impactpoint _impactnormal) (CallFunction|LineTrace))
  (CallFunction|SpawnPortalB _muzzleloc _impactpoint _impactpoint _impactnormal)
  (if (Variables|/Game/Blueprints/Player/FPSPawn_BP.FPSPawn_BP_C|GetAimDownSight _asfpspawn_bp)
    (Animation|Montage|PlayMontage _mesh1p "/Game/FPSPawn/Animations/Arms_AK_ADS_Fire_anim_Montage.Arms_AK_ADS_Fire_anim_Montage"
      (:then
        _))
    (else
      (Animation|Montage|PlayMontage _mesh1p "/Game/FPSPawn/Animations/Arms_AK_Fire_Montage.Arms_AK_Fire_Montage"
        (:then
          _))))
  (Utilities|MuzzleFlash))

(fn ConstructionScript
  (|CallParentFunction)
  (Variables|Default|SetMaxAmmo 0)
  (Variables|Default|SetAmmoCount 0)
  (Variables|Default|SetReloadTime 2.0)
  (Variables|Default|SetBulletSpread 0.0)
  (Variables|Default|SetName "NewEnumerator5")
  (Variables|Default|SetVariableMode false)
  (Variables|Default|SetStrenght 0.0)
  (Variables|Default|SetStrenghtKnockback 0.0)
  (Variables|Default|SetDamage 0))

(fn AmmoCheck
  (bind _returnvalue (Math|Random|RandomFloatinRange 0.7 1.2))
  (Math|Integer|DecrementInt (Variables|Default|GetAmmoCount)
    (:%20%20
      (Audio|PlaySoundatLocation "/Game/FPSPawn/SoundFX/Gunshot.Gunshot" (Transformation|GetWorldLocation (Variables|/Game/Blueprints/Player/FPSPawn_BP.FPSPawn_BP_C|GetFirstPersonCamera (.AsFPSPawn%20BP (Utilities|Casting|CastToFPSPawn_BP (Game|GetPlayerCharacter 0))))) "0, 0, 0" (+ _returnvalue 2.5) _returnvalue 0.0 "/Game/FPSPawn/SoundFX/AK_Attenuation.AK_Attenuation" "/Game/FPSPawn/SoundFX/AK_Concurrency.AK_Concurrency" 0)
      (Components|Animation|PlayAnimation (Variables|Default|GetPrimaryWeapon) "/Game/FPSPawn/Animations/AK_Fire_anim.AK_Fire_anim" false))))

(fn LineTrace
  (bind _returnvalue (Game|GetPlayerCharacter 0))
  (bind _bulletspread (Variables|Default|GetBulletSpread))
  (bind _returnvalue_2 (* _bulletspread -1.0))
  (bind _asfpspawn_bp (Utilities|Casting|CastToFPSPawn_BP _returnvalue))
  (bind _firstpersoncamera (Variables|/Game/Blueprints/Player/FPSPawn_BP.FPSPawn_BP_C|GetFirstPersonCamera _asfpspawn_bp))
  (bind _returnvalue_3 (Transformation|GetWorldLocation _firstpersoncamera))
  (bind _outhit (Collision|LineTraceByChannel (+ _returnvalue_3 (Variables|Default|GetAimOffset)) (+ (+ _returnvalue_3 (* (Math|Vector|GetForwardVector _firstpersoncamera) 2e+04)) (Math|Vector|MakeVector (Math|Random|RandomFloatinRange _returnvalue_2 _bulletspread) (Math|Random|RandomFloatinRange _returnvalue_2 _bulletspread) (Math|Random|RandomFloatinRange _returnvalue_2 _bulletspread))) "TraceTypeQuery1" false 0 "None")) ; Camera Shot
  (return (Transformation|GetWorldLocation (Variables|Default|GetMuzzle)) (.ImpactPoint (Collision|BreakHitResult _outhit)) (.ImpactNormal (Collision|BreakHitResult _outhit))))

(fn SpawnPortalA
  (params (Location :type Vector) (SpawnTransformLoc :type Vector) (Impact%20Point :type Vector) (Impact%20Normal :type Vector))
  (bind _returnvalue (Transformation|GetActorRightVector))
  (bind _returnvalue_2 (Game|GetPlayerCharacter 0))
  (bind _returnvalue_3 (* _returnvalue Impact%20Normal))
  (bind _asfpspawn_bp (Utilities|Casting|CastToFPSPawn_BP _returnvalue_2))
  (bind _portalb (Variables|/Game/Blueprints/Player/FPSPawn_BP.FPSPawn_BP_C|GetPortalB _asfpspawn_bp))
  (Utilities|IsValid (Variables|/Game/Blueprints/Player/FPSPawn_BP.FPSPawn_BP_C|GetPortalA _asfpspawn_bp)
    (:Is%20Valid
      (Actor|DestroyActor (Variables|/Game/Blueprints/Player/FPSPawn_BP.FPSPawn_BP_C|GetPortalA _asfpspawn_bp)))
    (:Is%20Not%20Valid
      _))
  (bind _returnvalue_4 (Game|SpawnActorfromClass "/Game/Blueprints/Props/PortalA.PortalA_C" (Math|Transform|MakeTransform SpawnTransformLoc (Math|Rotator|MakeRotationfromAxes _returnvalue_3 (* _returnvalue_3 Impact%20Normal) Impact%20Normal) "2.000000,2.000000,2.000000") "Undefined" 0 0))
  (bind _output_get (Variables|/Game/Blueprints/Player/FPSPawn_BP.FPSPawn_BP_C|SetPortalA _asfpspawn_bp _returnvalue_4))
  (Utilities|IsValid _portalb
    (:Is%20Valid
      (Rendering|Material|SetMaterial (Variables|/Game/Blueprints/Props/PortalB.PortalB_C|GetRenderTPA _portalb) 0 "/Game/Blueprints/Props/2Portal_Mat.2Portal_Mat")
      (Rendering|Material|SetMaterial (Variables|/Game/Blueprints/Props/PortalA.PortalA_C|GetRenderTPB _output_get) 0 "/Game/Blueprints/Props/1Portal_Mat.1Portal_Mat"))))

(fn SpawnPortalB
  (params (Location :type Vector) (SpawnTransformLoc :type Vector) (Impact%20Point :type Vector) (Impact%20Normal :type Vector))
  (bind _returnvalue (Transformation|GetActorRightVector))
  (bind _returnvalue_2 (Game|GetPlayerCharacter 0))
  (bind _returnvalue_3 (* _returnvalue Impact%20Normal))
  (bind _asfpspawn_bp (Utilities|Casting|CastToFPSPawn_BP _returnvalue_2))
  (bind _portala (Variables|/Game/Blueprints/Player/FPSPawn_BP.FPSPawn_BP_C|GetPortalA _asfpspawn_bp))
  (Utilities|IsValid (Variables|/Game/Blueprints/Player/FPSPawn_BP.FPSPawn_BP_C|GetPortalB _asfpspawn_bp)
    (:Is%20Valid
      (Actor|DestroyActor (Variables|/Game/Blueprints/Player/FPSPawn_BP.FPSPawn_BP_C|GetPortalB _asfpspawn_bp)))
    (:Is%20Not%20Valid
      _))
  (bind _returnvalue_4 (Game|SpawnActorfromClass "/Game/Blueprints/Props/PortalB.PortalB_C" (Math|Transform|MakeTransform SpawnTransformLoc (Math|Rotator|MakeRotationfromAxes _returnvalue_3 (* _returnvalue_3 Impact%20Normal) Impact%20Normal) "2.000000,2.000000,2.000000") "Undefined" 0 0))
  (bind _output_get (Variables|/Game/Blueprints/Player/FPSPawn_BP.FPSPawn_BP_C|SetPortalB _asfpspawn_bp _returnvalue_4))
  (Utilities|IsValid _portala
    (:Is%20Valid
      (Rendering|Material|SetMaterial (Variables|/Game/Blueprints/Props/PortalA.PortalA_C|GetRenderTPB _portala) 0 "/Game/Blueprints/Props/1Portal_Mat.1Portal_Mat")
      (Rendering|Material|SetMaterial (Variables|/Game/Blueprints/Props/PortalB.PortalB_C|GetRenderTPA _output_get) 0 "/Game/Blueprints/Props/2Portal_Mat.2Portal_Mat"))))