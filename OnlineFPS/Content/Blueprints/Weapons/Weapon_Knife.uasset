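; First-person knife weapon that doubles as the zombie infection attack, turning human players it hits into zombies when the wielder is one.
; Fire plays one of three random arm montages behind a short cooldown and runs a short camera trace with random spread.
; HitAction pushes Movable-tagged objects or applies infection, while SpawnDecalTracer places a knife decal oriented to the surface normal.
; Reload and dry-fire nodes remain unconnected.
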(event EventFire
  (bind _returnvalue (Game|GetPlayerCharacter 0))
  (bind _asfpspawn_bp (Utilities|Casting|CastToFPSPawn_BP _returnvalue))
  (bind _mesh1p (Variables|/Game/Blueprints/Player/FPSPawn_BP.FPSPawn_BP_C|GetMesh1P _asfpspawn_bp))
  (if (not (Variables|Default|GetCooldown))
    (Variables|Default|SetCooldown true)
    (Utilities|FlowControl|Sequence
      (:then_0
        (switch int (Math|Random|RandomIntegerinRange 0 2)
          (:0
            (Animation|Montage|PlayMontage _mesh1p "/Game/3D(MeshAndMaterials)/Animations/Arms_Knife_Attack_01_anim_Montage.Arms_Knife_Attack_01_anim_Montage"))
          (:1
            (Animation|Montage|PlayMontage _mesh1p "/Game/3D(MeshAndMaterials)/Animations/Arms_Knife_Attack_02_anim_Montage.Arms_Knife_Attack_02_anim_Montage"))
          (:2
            (Animation|Montage|PlayMontage _mesh1p "/Game/3D(MeshAndMaterials)/Animations/Arms_Knife_Attack_03_anim_Montage.Arms_Knife_Attack_03_anim_Montage"))))
      (:then_1
        (bind (_impactpoint _impactnormal) (CallFunction|LineTrace))
        (CallFunction|SpawnDecalTracer _impactpoint _impactnormal))
      (:then_2
        (Utilities|FlowControl|RetriggerableDelay 0.2)
        (Variables|Default|SetCooldown false)))))

(fn ConstructionScript
  (|CallParentFunction)
  (Variables|Default|SetName "NewEnumerator0")
  (Variables|Default|SetVariableMode false))

(fn LineTrace
  (bind _returnvalue (Game|GetPlayerCharacter 0))
  (bind _bulletspread (Variables|Default|GetBulletSpread))
  (bind _returnvalue_2 (* _bulletspread -1.0))
  (bind _asfpspawn_bp (Utilities|Casting|CastToFPSPawn_BP _returnvalue))
  (bind _firstpersoncamera (Variables|/Game/Blueprints/Player/FPSPawn_BP.FPSPawn_BP_C|GetFirstPersonCamera _asfpspawn_bp))
  (bind _returnvalue_3 (Transformation|GetWorldLocation _firstpersoncamera))
  (bind _outhit (Collision|LineTraceByChannel (+ _returnvalue_3 (Variables|Default|GetAimOffset)) (+ (+ _returnvalue_3 (* (Math|Vector|GetForwardVector _firstpersoncamera) 175.0)) (Math|Vector|MakeVector (Math|Random|RandomFloatinRange _returnvalue_2 _bulletspread) (Math|Random|RandomFloatinRange _returnvalue_2 _bulletspread) (Math|Random|RandomFloatinRange _returnvalue_2 _bulletspread))) "TraceTypeQuery1" false 0 "None")) ; Camera Shot
  (if (.bBlockingHit (Collision|BreakHitResult _outhit))
    (Utilities|HitAction (.ImpactPoint (Collision|BreakHitResult _outhit)) (.ImpactNormal (Collision|BreakHitResult _outhit)) (.HitActor (Collision|BreakHitResult _outhit)) (.HitComponent (Collision|BreakHitResult _outhit)) _asfpspawn_bp
      (:True
        _)
      (:False
        _))
    (return (.ImpactPoint (Collision|BreakHitResult _outhit)) (.ImpactNormal (Collision|BreakHitResult _outhit)))))

(fn SpawnDecalTracer
  (params (Impact%20Point :type Vector) (ImpactNormal :type Vector))
  (bind _returnvalue (Math|Conversions|RotationFromXVector ImpactNormal))
  (bind _returnvalue_2 (Game|GetPlayerCharacter 0))
  (bind _asfpspawn_bp (Utilities|Casting|CastToFPSPawn_BP _returnvalue_2))
  (bind _firstpersoncamera (Variables|/Game/Blueprints/Player/FPSPawn_BP.FPSPawn_BP_C|GetFirstPersonCamera _asfpspawn_bp))
  (if (Math|Vector|Equal(Vector) ImpactNormal "0, 0,1.000000" 0.0001)
    (Game|SpawnActorfromClass "/Game/Blueprints/Weapons/KnifeDecal_BP.KnifeDecal_BP_C" (Math|Transform|MakeTransform Impact%20Point (Math|Rotator|MakeRotator -9e+01 9e+01 (.yaw (Math|Conversions|RotationFromXVector (Math|Vector|GetForwardVector _firstpersoncamera)))) "0.100000,0.080000,0.080000") "Undefined" 0 0)
    (else
      (Game|SpawnActorfromClass "/Game/Blueprints/Weapons/KnifeDecal_BP.KnifeDecal_BP_C" (Math|Transform|MakeTransform Impact%20Point (Math|Rotator|MakeRotator (+ (.roll (Transformation|GetWorldRotation _firstpersoncamera)) 9e+01) (.pitch _returnvalue) (+ (.yaw _returnvalue) 1.8e+02)) "0.100000,0.080000,0.080000") "Undefined" 0 0)))
  (return))