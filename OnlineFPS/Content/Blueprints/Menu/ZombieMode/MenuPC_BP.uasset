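; Player controller for the Zombie mode menu that creates the menu HUD and handles multiplayer session hosting, searching and joining.
; BeginPlay creates the widget once and shows a locked cursor in Game and UI input.
; Host creates a LAN session and opens the wait map as a listen server.
; Search runs a non-LAN query listing results as HUD_Session widgets, while joining uses a search result or an IP console command.
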(event Custom|Search
  ;[0 1 0.3467] Search and Join Session By IP (no need to specify IP address
  (Widget|Panel|ClearChildren (Variables|/Game/HUD/Menu_HUD/HUD_Menu_Zombie.HUD_Menu_Zombie_C|GetBox_SessionDisplay (Variables|Default|GetHudMenu_Var)))
  (Variables|Default|SetIsLookingForSession true)
  (bind _results (|FindSessions self 4 false)
    (:OnSuccess
      (for _array_element _results
        (bind _returnvalue (UserInterface|CreateWidget "/Game/HUD/Menu_HUD/HUD_Session.HUD_Session_C" 0 _array_element))
        (Widget|Panel|AddChild (Variables|/Game/HUD/Menu_HUD/HUD_Menu_Zombie.HUD_Menu_Zombie_C|GetBox_SessionDisplay (Variables|Default|GetHudMenu_Var)) _returnvalue))
      (Variables|Default|SetIsLookingForSession false))))

(event Custom|Host
  ;[1 0.8712 0] Host your Session
  (|Session self 10 true
    (:OnSuccess
      (Game|OpenLevel(byName) "WaitScreen_Map" true "listen"))))

(event Custom|Join
  (params (IP_Address :type String))
  ;[1 0 0.7734] Join Session By IP
  (Development|ExecuteConsoleCommand (Utilities|String|Append "open " IP_Address) 0))

(event Custom|Join%20Session
  (params (SearchResult :type Blueprint%20Session%20Result%20Structure%20%28by%20ref%29))
  ;[1 0 0.6328] Join the Sesion when find (RightButton)
  (|JoinSession self SearchResult))

(event EventBeginPlay
  ;[0 1 0.8125] Create HUD and Init Cursor
  (CallFunction|HUDMenu)
  (CallFunction|InitCursor))

(fn ConstructionScript)

(fn HUDMenu
  ;[0 0.9766 1] Courte vérifaction pour eviter la double création du widget
  (Utilities|IsValid (Variables|Default|GetHudMenu_Var)
    (:Is%20Not%20Valid
      (bind _returnvalue (UserInterface|CreateWidget "/Game/HUD/Menu_HUD/HUD_Menu_Zombie.HUD_Menu_Zombie_C"))
      (bind _output_get (Variables|Default|SetHudMenu_Var _returnvalue))
      (UserInterface|Viewport|AddtoViewport _output_get 0))))

(fn InitCursor
  (bind _returnvalue (Game|GetCurrentLevelName true))
  (if (Utilities|Enum|Equal(Enum) _returnvalue "MenuMap")
    (Variables|Default|SetbShowMouseCursor true)
    (Input|SetInputModeGameandUI self 0 "LockAlways" true)
    (else
      (Variables|Default|SetbShowMouseCursor true)
      (Input|SetInputModeGameandUI self 0 "LockAlways" true))))

(fn OnRepHudMenuVar)