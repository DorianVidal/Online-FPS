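; ChoosePC_BP is a player controller for the Choose menu that puts the game mode selection HUD on screen.
; BeginPlay creates the HUD_GameMode widget if none is stored, caches it and adds it to the viewport.
; InitCursor shows the mouse and sets Game and UI input with the mouse always locked; its ChooseMode_Map level check has identical branches, and nothing in this file calls it.
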(event EventBeginPlay
  (Utilities|IsValid (Variables|Default|GetHUD_GameMode_Var)
    (:Is%20Not%20Valid
      (bind _returnvalue (UserInterface|CreateWidget "/Game/HUD/HUD_GameMode.HUD_GameMode_C"))
      (bind _output_get (Variables|Default|SetHUD_GameMode_Var _returnvalue))
      (UserInterface|Viewport|AddtoViewport _output_get 0))))

(fn ConstructionScript)

(fn InitCursor
  (bind _returnvalue (Game|GetCurrentLevelName true))
  (if (Utilities|Enum|Equal(Enum) _returnvalue "ChooseMode_Map")
    (Variables|Default|SetbShowMouseCursor true)
    (Input|SetInputModeGameandUI self 0 "LockAlways" true)
    (else
      (Variables|Default|SetbShowMouseCursor true)
      (Input|SetInputModeGameandUI self 0 "LockAlways" true))))