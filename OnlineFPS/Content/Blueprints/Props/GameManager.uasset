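; GameManager is a Blueprint that starts the infection phase by turning a random player pawn into a zombie after a countdown.
; Tick decrements TimeBeforeInfection by delta time until it runs out.
; A DoOnce then gathers all FPSPawn_BP actors in the level and calls BecomeZombie on one chosen at random.
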(event EventBeginPlay)

(event Collision|EventActorBeginOverlap
  (params (OtherActor :type Actor%20Object%20Reference)))

(event EventTick
  (params (DeltaSeconds :type Float%20%28single-precision%29))
  (if (> (Variables|Default|GetTimeBeforeInfection) 0.0)
    (Variables|Default|SetTimeBeforeInfection (- (Variables|Default|GetTimeBeforeInfection) DeltaSeconds))
    (else
      (Utilities|FlowControl|DoOnce false
        (:Completed
          (bind _outactors (Actor|GetAllActorsOfClass "/Game/Blueprints/Player/FPSPawn_BP.FPSPawn_BP_C"))
          (Default|BecomeZombie (Utilities|Array|Get(acopy) _outactors (Math|Random|RandomIntegerinRange 0 (- (Utilities|Array|Length _outactors) 1)))))))))

(fn ConstructionScript)