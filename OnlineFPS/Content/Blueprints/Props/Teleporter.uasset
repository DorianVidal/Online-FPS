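; Teleporter prop with two linked portals that move overlapping actors between each other and drive see-through portal views.
; Overlapping either portal box teleports the actor to the other box, with a shared flag and short delay preventing an immediate bounce back.
; Each tick, two capture components mirror the player camera's rotation and its position shifted by the offset between portals, without compensating for portal rotation.
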(event OnComponentHit(1PortalBox)
  (params (HitComponent :type Primitive%20Component%20Object%20Reference) (OtherActor :type Actor%20Object%20Reference) (OtherComp :type Primitive%20Component%20Object%20Reference) (NormalImpulse :type Vector :default "0, 0, 0") (Hit :type Hit%20Result%20Structure%20%28by%20ref%29)))

(event OnComponentBeginOverlap(RenderTP2)
  (params (OverlappedComponent :type Primitive%20Component%20Object%20Reference) (OtherActor :type Actor%20Object%20Reference) (OtherComp :type Primitive%20Component%20Object%20Reference) (OtherBodyIndex :type Integer) (bFromSweep :type Boolean) (SweepResult :type Hit%20Result%20Structure%20%28by%20ref%29)))

(event OnComponentBeginOverlap(2PortalBox)
  (params (OverlappedComponent :type Primitive%20Component%20Object%20Reference) (OtherActor :type Actor%20Object%20Reference) (OtherComp :type Primitive%20Component%20Object%20Reference) (OtherBodyIndex :type Integer) (bFromSweep :type Boolean) (SweepResult :type Hit%20Result%20Structure%20%28by%20ref%29))
  ;[1 0 0.6328] Portal2 TP
  (if (Variables|Default|GetCanTeleport)
    (Variables|Default|SetCanTeleport false)
    (Transformation|SetActorLocation OtherActor (Transformation|GetWorldLocation (Variables|Default|Get1PortalBox)) false true)
    (Utilities|FlowControl|Delay 0.5)
    (Variables|Default|SetCanTeleport true)))

(event OnComponentBeginOverlap(1PortalBox)
  (params (OverlappedComponent :type Primitive%20Component%20Object%20Reference) (OtherActor :type Actor%20Object%20Reference) (OtherComp :type Primitive%20Component%20Object%20Reference) (OtherBodyIndex :type Integer) (bFromSweep :type Boolean) (SweepResult :type Hit%20Result%20Structure%20%28by%20ref%29))
  ;[0 0.7422 1] Portal1 TP
  (if (Variables|Default|GetCanTeleport)
    (Variables|Default|SetCanTeleport false)
    (Transformation|SetActorLocation OtherActor (Transformation|GetWorldLocation (Variables|Default|Get2PortalBox)) false true)
    (Utilities|FlowControl|Delay 0.5)
    (Variables|Default|SetCanTeleport true)))

(event EventBeginPlay)

(event Collision|EventActorBeginOverlap
  (params (OtherActor :type Actor%20Object%20Reference)))

(event EventTick
  (params (DeltaSeconds :type Float%20%28single-precision%29))
  (bind _returnvalue (Game|GetPlayerController 0))
  (bind _returnvalue_2 (Game|GetPlayerController 0))
  (bind _playercameramanager (Variables|/Script/Engine.PlayerController|GetPlayerCameraManager _returnvalue))
  (bind _playercameramanager_2 (Variables|/Script/Engine.PlayerController|GetPlayerCameraManager _returnvalue_2))
  (bind _transformcomponent (Variables|/Script/Engine.PlayerCameraManager|GetTransformComponent _playercameramanager))
  (bind _transformcomponent_2 (Variables|/Script/Engine.PlayerCameraManager|GetTransformComponent _playercameramanager_2))
  (Transformation|SetWorldLocationAndRotation (Variables|Default|GetCaptureInTP1) (+ (Transformation|GetWorldLocation _transformcomponent_2) (- (Transformation|GetWorldLocation (Variables|Default|GetPortalA)) (Transformation|GetWorldLocation (Variables|Default|GetPortalB)))) (Transformation|GetWorldRotation _transformcomponent_2) false false)
  (Transformation|SetWorldLocationAndRotation (Variables|Default|GetCaptureInTP2) (+ (Transformation|GetWorldLocation _transformcomponent) (- (Transformation|GetWorldLocation (Variables|Default|GetPortalB)) (Transformation|GetWorldLocation (Variables|Default|GetPortalA)))) (Transformation|GetWorldRotation _transformcomponent) false false))

(fn ConstructionScript)