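; PortalA is a portal prop that teleports any overlapping actor to the location of the linked PortalB.
; On overlap it reads PortalB from the player's FPSPawn_BP and proceeds only if that portal is valid.
; The pawn's CanTeleport flag acts as a shared lock, cleared before the unswept move and restored after a short delay.
; Only location is set, with no change to rotation.
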(event Collision|EventActorBeginOverlap
  (params (OtherActor :type Actor%20Object%20Reference))
  (bind _returnvalue (Game|Player|GetPlayerPawn 0))
  (bind _asfpspawn_bp (Utilities|Casting|CastToFPSPawn_BP _returnvalue))
  (bind _portalb (Variables|/Game/Blueprints/Player/FPSPawn_BP.FPSPawn_BP_C|GetPortalB _asfpspawn_bp))
  (if (Utilities|IsValid _portalb)
    (if (Variables|/Game/Blueprints/Player/FPSPawn_BP.FPSPawn_BP_C|GetCanTeleport _asfpspawn_bp)
      (Variables|/Game/Blueprints/Player/FPSPawn_BP.FPSPawn_BP_C|SetCanTeleport _asfpspawn_bp false)
      (Transformation|SetActorLocation OtherActor (Transformation|GetWorldLocation (Variables|/Script/Engine.Actor|GetRootComponent _portalb)) false true)
      (Utilities|FlowControl|Delay 0.5)
      (Variables|/Game/Blueprints/Player/FPSPawn_BP.FPSPawn_BP_C|SetCanTeleport _asfpspawn_bp true))))

(fn ConstructionScript)