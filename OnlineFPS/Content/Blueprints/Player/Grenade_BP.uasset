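; Grenade actor Blueprint that launches its Sphere component with a physics impulse when the Collider component wakes.
; The wake event applies a fixed-strength impulse at the Sphere's location, directed along the waking component's normalized world position, then prints a debug "Hello".
; BeginPlay only runs a repeating delay with no other action, and no detonation or damage logic is present.
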(event OnComponentWake(collider)
  (params (WakingComponent :type Primitive%20Component%20Object%20Reference) (BoneName :type Name :default "None"))
  (Physics|AddImpulseatLocation (Variables|Default|GetSphere) (* (Math|Vector|Normalize (Transformation|GetWorldLocation WakingComponent)) 1e+03) (Transformation|GetWorldLocation (Variables|Default|GetSphere)) "None")
  (Development|PrintString "Hello"))

(event EventBeginPlay
  (Utilities|FlowControl|Sequence :!label _label
    (:then_0
      (Utilities|FlowControl|Delay 5.0)
      (goto _label))))

(event Collision|EventActorBeginOverlap
  (params (OtherActor :type Actor%20Object%20Reference)))

(event EventTick
  (params (DeltaSeconds :type Float%20%28single-precision%29)))

(fn ConstructionScript)