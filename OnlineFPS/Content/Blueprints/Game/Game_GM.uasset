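; Game mode for an FPS that handles pawn respawning at player starts.
; On BeginPlay it caches all PlayerStart actors and numbers existing FPSPawn_BP pawns through their PlayerControllerID.
; SpawnCharacter and DespawnCharacter are identical: each destroys a controller's valid pawn, then spawns and possesses a new FPSPawn_BP at GetRandomSpawn's transform.
; GetRandomSpawn's graph contains a random pick from the cached starts, shown as unconnected.
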(event Custom|DespawnCharacter
  (params (PlayerController :type Player%20Controller%20Object%20Reference))
  (bind _returnvalue (Pawn|GetControlledPawn PlayerController))
  (Utilities|IsValid _returnvalue
    (:Is%20Valid
      (Actor|DestroyActor _returnvalue)
      (bind _returnvalue_2 (Game|SpawnActorfromClass "/Game/Blueprints/Player/FPSPawn_BP.FPSPawn_BP_C" (Utilities|GetRandomSpawn) "Undefined" 0 0))
      (Pawn|Possess PlayerController _returnvalue_2))))

(event Custom|SpawnCharacter
  (params (PlayerController :type Player%20Controller%20Object%20Reference))
  (bind _returnvalue (Pawn|GetControlledPawn PlayerController))
  (Utilities|IsValid _returnvalue
    (:Is%20Valid
      (Actor|DestroyActor _returnvalue)
      (bind _returnvalue_2 (Game|SpawnActorfromClass "/Game/Blueprints/Player/FPSPawn_BP.FPSPawn_BP_C" (Utilities|GetRandomSpawn) "Undefined" 0 0))
      (Pawn|Possess PlayerController _returnvalue_2))))

(event EventBeginPlay
  (bind _outactors (Actor|GetAllActorsOfClass "/Script/Engine.PlayerStart"))
  (Variables|Default|SetSpawnPoints _outactors)
  (bind _outactors_2 (Actor|GetAllActorsOfClass "/Game/Blueprints/Player/FPSPawn_BP.FPSPawn_BP_C"))
  (for (_array_element _array_index) _outactors_2
    (Variables|/Game/Blueprints/Player/FPSPawn_BP.FPSPawn_BP_C|SetPlayerControllerID _array_element _array_index)))

(event EventTick
  (params (DeltaSeconds :type Float%20%28single-precision%29)))

(fn ConstructionScript)