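; FPSPC_PB is an FPS player controller Blueprint that handles text chat between players.
; On BeginPlay it names itself "Player" plus a random number, which is not checked for uniqueness.
; SendMessage prefixes the text with that name and calls ReceiveMessage on every FPSPC_PB instance found through GetAllActorsOfClass.
; ReceiveMessage casts the controller's HUD to FPS_HUD and passes the text to its chat window.
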(event Custom|SendMessage
  (params (Message :type Text))
  ;[0 1 0.1797] Envoyer un message
  (bind _outactors (Actor|GetAllActorsOfClass "FPSPC_PB_C"))
  (for _array_element _outactors
    (CallFunction|ReceiveMessage _array_element (Utilities|Text|ToText(String) (Utilities|String|Append (Variables|Default|GetPlayerName) " : " (Utilities|String|ToString(Text) Message))))))

(event Custom|ReceiveMessage
  (params (Message :type Text))
  ;[0.2188 0 1] Recevoir un Message
  (bind _asfps_hud (Utilities|Casting|CastToFPS_HUD (HUD|GetHUD)))
  (Default|UpdateChat (Variables|/Game/Blueprints/Player/FPS_HUD.FPS_HUD_C|GetChatWindowsVar _asfps_hud) Message))

(event EventBeginPlay
  ;[1 0.2344 0] Generate Name
  (Variables|Default|SetPlayerName (Utilities|String|Append "Player" (Utilities|String|ToString(Integer) (Math|Random|RandomIntegerinRange 1 10)))))

(fn ConstructionScript)